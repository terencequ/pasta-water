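; Player controller that turns input into camera look, movement and jumping for the pasta water character.
; On possess it caches the pawn and a cast BP_PastaWaterCharacter, printing a warning if the cast fails, and clears both references on unpossess.
; Look axes apply mouse sensitivity, movement follows the control rotation's yaw only, and jump calls the cached character.
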(event EventBeginPlay)

(event EventTick
  (params (DeltaSeconds :type Float%20%28single-precision%29)))

(event EventPossess
  (params (PossessedPawn :type Pawn%20Object%20Reference))
  (bind _output_get (Variables|Default|SetControlling%20Pawn PossessedPawn))
  (bind _asbp_pasta_water_character (Utilities|Casting|CastToBP_PastaWaterCharacter _output_get)
    (:then
      (Variables|Default|SetControlling%20Pasta%20Water%20Character _asbp_pasta_water_character))
    (:CastFailed
      (Development|PrintString "Not possessing a pasta water character!"))))

(event EventUnPossess
  (params (UnpossessedPawn :type Pawn%20Object%20Reference))
  (Variables|Default|SetControlling%20Pawn 0)
  (Variables|Default|SetControlling%20Pasta%20Water%20Character 0))

(event Input|ActionEvents|InputActionJump
  (params (Key :type Key%20Structure :default "None"))
  ;[1 1 1] Movement
  (:Pressed
    (CallFunction|InputJump)))

(event Input|AxisEvents|InputAxisLookPitch
  (params (AxisValue :type Float%20%28single-precision%29))
  ;[1 1 1] Looking
  (CallFunction|InputLookPitch AxisValue))

(event Input|AxisEvents|InputAxisLookYaw
  (params (AxisValue :type Float%20%28single-precision%29))
  ;[1 1 1] Looking
  (CallFunction|InputLookYaw AxisValue))

(event Input|AxisEvents|InputAxisMoveForwardBackward
  (params (AxisValue :type Float%20%28single-precision%29))
  ;[1 1 1] Movement
  (CallFunction|InputForwardBackward AxisValue))

(event Input|AxisEvents|InputAxisMoveRightLeft
  (params (AxisValue :type Float%20%28single-precision%29))
  ;[1 1 1] Movement
  (CallFunction|InputRightLeft AxisValue))

(fn ConstructionScript)

(fn InputLookPitch
  (params (Input%20Value :type Float%20%28single-precision%29))
  (Class|PlayerController|AddPitchInput (* Input%20Value (Variables|Default|GetMouse%20Pitch%20Sensitivity))))

(fn InputLookYaw
  (params (Input%20Value :type Float%20%28single-precision%29))
  (Class|PlayerController|AddYawInput (* Input%20Value (Variables|Default|GetMouse%20Yaw%20Sensitivity))))

(fn InputRightLeft
  (params (Input%20Value :type Float%20%28single-precision%29))
  (Pawn|Input|AddMovementInput (Variables|Default|GetControlling%20Pawn) (Math|Vector|GetRightVector (CallFunction|GetYawControlRotation)) Input%20Value false))

(fn InputForwardBackward
  (params (Input%20Value :type Float%20%28single-precision%29))
  (Pawn|Input|AddMovementInput (Variables|Default|GetControlling%20Pawn) (Math|Vector|GetForwardVector (CallFunction|GetYawControlRotation)) Input%20Value false))

(fn InputJump
  (Character|Jump (Variables|Default|GetControlling%20Pasta%20Water%20Character)))

(fn GetYawControlRotation
  (return (Math|Rotator|MakeRotator 0.0 0.0 (.Yaw (Math|Rotator|BreakRotator (Pawn|GetControlRotation :!class /Script/Engine.Controller))))))