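; BP_PlayerInventoryAC is the player's inventory component, meant to sit on a Player Controller, that manages the on-screen inventory UI.
; On BeginPlay it caches the owning controller, printing a warning if the cast fails, then creates a WBP_PlayerInventory widget and adds it hidden to the viewport.
; ToggleInventory delegates to the widget's ToggleWidget, and a debug function prints each item stack's item details.
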(event Custom|Toggle%20Inventory
  (Default|ToggleWidget (Variables|Default|GetInventory%20Widget)))

(event EventBeginPlay
  (CallFunction|SetupPlayerController)
  (CallFunction|SetupInventoryWidget))

(event EventTick
  (params (DeltaSeconds :type Float%20%28single-precision%29)))

(fn SetupPlayerController
  (bind _asplayer_controller (Utilities|Casting|CastToPlayerController (Components|GetOwner))
    (:then
      (Variables|Default|SetPlayer%20Controller _asplayer_controller))
    (:CastFailed
      (Development|PrintString "BP_PlayerInventoryAC needs to have a Player Controller as a parent!"))))

(fn SetupInventoryWidget
  (bind _returnvalue (UserInterface|CreateWidget "/Game/Game/Inventory/Widgets/WBP_PlayerInventory.WBP_PlayerInventory_C" (Variables|Default|GetPlayer%20Controller)))
  (Variables|Default|SetInventory%20Widget _returnvalue)
  (Widget|SetVisibility (Variables|Default|GetInventory%20Widget) "Hidden")
  (UserInterface|Viewport|AddtoViewport (Variables|Default|GetInventory%20Widget) 0)
  (return (Variables|Default|GetInventory%20Widget)))

(fn PrintInventoryContents
  (for _array_element (Class|PlayerInventoryAC|GetAllItemStacksImplementation)
    (Development|PrintString (Utilities|String|JoinStringArray (Utilities|Array|MakeArray (.Id (Utilities|Struct|BreakItem (.Item (Utilities|Struct|BreakItemStack _array_element)))) (.Name (Utilities|Struct|BreakItem (.Item (Utilities|Struct|BreakItemStack _array_element)))) (Utilities|String|ToString(Integer) (.MaxStackQuantity (Utilities|Struct|BreakItem (.Item (Utilities|Struct|BreakItemStack _array_element)))))) ","))))